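; Road actor that builds a procedural road mesh from a Centerline string in its construction script.
; It splits the string on semicolons into 2D points, swapping and negating the two coordinates of each.
; It then resets the RoadMesh dynamic mesh and uses Geometry Script to append a thin box per segment, centered between neighboring points, yawed along them and WidthCm wide.
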(event EventBeginPlay)

(event Collision|EventActorBeginOverlap
  (params (OtherActor :type Actor%20Object%20Reference)))

(event EventTick
  (params (DeltaSeconds :type Float%20%28single-precision%29)))

(fn ConstructionScript
  (bind _temproadpoints (Variables|Default|GetTempRoadPoints))
  (bind _temproadpoints_2 (Variables|Default|GetTempRoadPoints))
  (bind _returnvalue (Utilities|Array|Length _temproadpoints_2))
  (bind _returnvalue_2 (DynamicMeshComponent|GetDynamicMesh (Variables|Default|GetRoadMesh)))
  (bind _returnvalue_3 (DynamicMesh|Reset _returnvalue_2))
  (Utilities|Array|Clear (Variables|Default|GetTempRoadPoints))
  (for _array_element (Utilities|String|ParseIntoArray (Variables|Default|Getcenterline) ";")
    (Utilities|Array|Add (Variables|Default|GetTempRoadPoints) (Math|Vector2D|MakeVector2D (* (Math|Conversions|ToFloat(Integer) (Utilities|Array|Get(acopy) (Utilities|String|ParseIntoArray _array_element " ") 1)) -1.0) (* (Math|Conversions|ToFloat(Integer) (Utilities|Array|Get(acopy) (Utilities|String|ParseIntoArray _array_element " "))) -1.0))))
  (if (>= _returnvalue 2)
    (for _index (range 0 (- _returnvalue 2))
      (Class|GeometryScriptLibraryMeshPrimitiveFunctions|AppendBox :TargetMesh _returnvalue_3 :Transform (Math|Transform|MakeTransform (Math|Vector|MakeVector (/ (+ (.X (Math|Vector2D|BreakVector2D (Utilities|Array|Get(acopy) _temproadpoints _index))) (.X (Math|Vector2D|BreakVector2D (Utilities|Array|Get(acopy) _temproadpoints (+ _index 1))))) 2.0) (/ (+ (.Y (Math|Vector2D|BreakVector2D (Utilities|Array|Get(acopy) _temproadpoints _index))) (.Y (Math|Vector2D|BreakVector2D (Utilities|Array|Get(acopy) _temproadpoints (+ _index 1))))) 2.0) 5.0) (Math|Rotator|MakeRotator 0.0 0.0 (Class|KismetMathLibrary|DegAtan2 (- (.Y (Math|Vector2D|BreakVector2D (Utilities|Array|Get(acopy) _temproadpoints (+ _index 1)))) (.Y (Math|Vector2D|BreakVector2D (Utilities|Array|Get(acopy) _temproadpoints _index)))) (- (.X (Math|Vector2D|BreakVector2D (Utilities|Array|Get(acopy) _temproadpoints (+ _index 1)))) (.X (Math|Vector2D|BreakVector2D (Utilities|Array|Get(acopy) _temproadpoints _index))))))) :DimensionX (Math|Float|Sqrt (+ (* (- (.X (Math|Vector2D|BreakVector2D (Utilities|Array|Get(acopy) _temproadpoints (+ _index 1)))) (.X (Math|Vector2D|BreakVector2D (Utilities|Array|Get(acopy) _temproadpoints _index)))) (- (.X (Math|Vector2D|BreakVector2D (Utilities|Array|Get(acopy) _temproadpoints (+ _index 1)))) (.X (Math|Vector2D|BreakVector2D (Utilities|Array|Get(acopy) _temproadpoints _index))))) (* (- (.Y (Math|Vector2D|BreakVector2D (Utilities|Array|Get(acopy) _temproadpoints (+ _index 1)))) (.Y (Math|Vector2D|BreakVector2D (Utilities|Array|Get(acopy) _temproadpoints _index)))) (- (.Y (Math|Vector2D|BreakVector2D (Utilities|Array|Get(acopy) _temproadpoints (+ _index 1)))) (.Y (Math|Vector2D|BreakVector2D (Utilities|Array|Get(acopy) _temproadpoints _index))))))) :DimensionY (Variables|Default|Getwidth_cm) :DimensionZ 1e+01 :Origin "Center"))))