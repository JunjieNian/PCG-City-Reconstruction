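; Generates a city of buildings and roads from data tables as a single dynamic mesh, rebuilt in the construction script.
; Each building's vertices are gathered by ID from a separate vertex table, with Y negated, and extruded to that building's height with Geometry Script.
; Road points are gathered the same way, and each segment becomes a thin box at the road's width, centred between its endpoints and yawed along it.
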(event EventBeginPlay)

(event Collision|EventActorBeginOverlap
  (params (OtherActor :type Actor%20Object%20Reference)))

(event EventTick
  (params (DeltaSeconds :type Float%20%28single-precision%29)))

(fn ConstructionScript
  (bind _roadsmeta (Variables|Default|GetRoadsMeta))
  (bind _roadsvert (Variables|Default|GetRoadsVert))
  (bind _temproadpoints (Variables|Default|GetTempRoadPoints))
  (bind _temproadpoints_2 (Variables|Default|GetTempRoadPoints))
  (bind _returnvalue (Utilities|Array|Length _temproadpoints))
  (bind _returnvalue_2 (DynamicMeshComponent|GetDynamicMesh (Variables|Default|GetCityMesh)))
  (bind _output_get (Variables|Default|SetTargetMesh _returnvalue_2))
  (DynamicMesh|Reset _output_get)
  (bind _outrownames (DataTable|GetDataTableRowNames (Variables|Default|GetBuildingsMeta)))
  (for _array_element _outrownames
    (bind _returnvalue_3 (Utilities|GetDataTableRow (Variables|Default|GetBuildingsMeta) _array_element)
      (:then
        (if true
          (Variables|Default|SetCurrentBuildingId (.building_id (Utilities|Struct|BreakS_BuildingMeta _returnvalue_3)))
          (Variables|Default|SetCurrentHeightCm (.height_cm (Utilities|Struct|BreakS_BuildingMeta _returnvalue_3)))
          (Utilities|Array|Clear (Variables|Default|GetTempFootprint))
          (bind _outrownames_2 (DataTable|GetDataTableRowNames (Variables|Default|GetBuildingsVert)))
          (for _array_element_2 _outrownames_2
            (bind _returnvalue_4 (Utilities|GetDataTableRow (Variables|Default|GetBuildingsVert) _array_element_2)
              (:then
                (if (== (.building_id (Utilities|Struct|BreakS_BuildingVert _returnvalue_4)) (Variables|Default|GetCurrentBuildingId))
                  (Utilities|Array|Add (Variables|Default|GetTempFootprint) (Math|Vector2D|MakeVector2D (.x_cm (Utilities|Struct|BreakS_BuildingVert _returnvalue_4)) (* (.y_cm (Utilities|Struct|BreakS_BuildingVert _returnvalue_4)) -1.0)))))))
          (if (>= (Utilities|Array|Length (Variables|Default|GetTempFootprint)) 3)
            (Class|GeometryScriptLibraryMeshPrimitiveFunctions|AppendSimpleExtrudePolygon :TargetMesh (Variables|Default|GetTargetMesh) :Transform (Math|Transform|MakeTransform "0, 0, 0") :PolygonVertices (Variables|Default|GetTempFootprint) :Height (Variables|Default|GetCurrentHeightCm) :HeightSteps 1))))))
  (bind _outrownames_3 (DataTable|GetDataTableRowNames _roadsmeta))
  (for _array_element_3 _outrownames_3
    (bind _returnvalue_5 (Utilities|GetDataTableRow _roadsmeta _array_element_3)
      (:then
        (Variables|Default|SetCurrentRoadId (.road_id (Utilities|Struct|BreakS_RoadMeta _returnvalue_5)))
        (Variables|Default|SetCurrentRoadWidthCm (.width_cm (Utilities|Struct|BreakS_RoadMeta _returnvalue_5)))
        (Utilities|Array|Clear (Variables|Default|GetTempRoadPoints))
        (bind _outrownames_4 (DataTable|GetDataTableRowNames _roadsvert))
        (for _array_element_4 _outrownames_4
          (bind _returnvalue_6 (Utilities|GetDataTableRow _roadsvert _array_element_4)
            (:then
              (if (== (Variables|Default|GetCurrentRoadId) (.road_id (Utilities|Struct|BreakS_RoadVert _returnvalue_6)))
                (Utilities|Array|Add (Variables|Default|GetTempRoadPoints) (Math|Vector2D|MakeVector2D (.x_cm (Utilities|Struct|BreakS_RoadVert _returnvalue_6)) (* (.y_cm (Utilities|Struct|BreakS_RoadVert _returnvalue_6)) -1.0)))))))
        (if (>= _returnvalue 2)
          (for _index (range 0 (- _returnvalue 2))
            (Class|GeometryScriptLibraryMeshPrimitiveFunctions|AppendBox :TargetMesh (Variables|Default|GetTargetMesh) :Transform (Math|Transform|MakeTransform (Math|Vector|MakeVector (/ (+ (.X (Math|Vector2D|BreakVector2D (Utilities|Array|Get(acopy) _temproadpoints_2 _index))) (.X (Math|Vector2D|BreakVector2D (Utilities|Array|Get(acopy) _temproadpoints_2 (+ _index 1))))) 2.0) (/ (+ (.Y (Math|Vector2D|BreakVector2D (Utilities|Array|Get(acopy) _temproadpoints_2 _index))) (.Y (Math|Vector2D|BreakVector2D (Utilities|Array|Get(acopy) _temproadpoints_2 (+ _index 1))))) 2.0) 5.0) (Math|Rotator|MakeRotator 0.0 0.0 (Class|KismetMathLibrary|DegAtan2 (- (.Y (Math|Vector2D|BreakVector2D (Utilities|Array|Get(acopy) _temproadpoints_2 (+ _index 1)))) (.Y (Math|Vector2D|BreakVector2D (Utilities|Array|Get(acopy) _temproadpoints_2 _index)))) (- (.X (Math|Vector2D|BreakVector2D (Utilities|Array|Get(acopy) _temproadpoints_2 (+ _index 1)))) (.X (Math|Vector2D|BreakVector2D (Utilities|Array|Get(acopy) _temproadpoints_2 _index))))))) :DimensionX (Math|Float|Sqrt (+ (* (- (.X (Math|Vector2D|BreakVector2D (Utilities|Array|Get(acopy) _temproadpoints_2 (+ _index 1)))) (.X (Math|Vector2D|BreakVector2D (Utilities|Array|Get(acopy) _temproadpoints_2 _index)))) (- (.X (Math|Vector2D|BreakVector2D (Utilities|Array|Get(acopy) _temproadpoints_2 (+ _index 1)))) (.X (Math|Vector2D|BreakVector2D (Utilities|Array|Get(acopy) _temproadpoints_2 _index))))) (* (- (.Y (Math|Vector2D|BreakVector2D (Utilities|Array|Get(acopy) _temproadpoints_2 (+ _index 1)))) (.Y (Math|Vector2D|BreakVector2D (Utilities|Array|Get(acopy) _temproadpoints_2 _index)))) (- (.Y (Math|Vector2D|BreakVector2D (Utilities|Array|Get(acopy) _temproadpoints_2 (+ _index 1)))) (.Y (Math|Vector2D|BreakVector2D (Utilities|Array|Get(acopy) _temproadpoints_2 _index))))))) :DimensionY (Variables|Default|GetCurrentRoadWidthCm) :DimensionZ 1e+01 :Origin "Center")))))))