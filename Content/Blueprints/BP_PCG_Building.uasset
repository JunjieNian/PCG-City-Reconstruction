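; BP_PCG_Building is a procedural building actor that generates a simple extruded mesh from a footprint string and a height.
; The construction script resets the BuildingMesh dynamic mesh and parses the semicolon-separated Footprint into 2D points, swapping and negating the two coordinates.
; With at least three points, Geometry Script extrudes the polygon to HeightCm in a single step.
; The event graph holds no active logic.
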(event EventBeginPlay)

(event Collision|EventActorBeginOverlap
  (params (OtherActor :type Actor%20Object%20Reference)))

(event EventTick
  (params (DeltaSeconds :type Float%20%28single-precision%29)))

(fn ConstructionScript
  (bind _tempfootprint (Variables|Default|GetTempFootprint))
  (bind _returnvalue (DynamicMeshComponent|GetDynamicMesh (Variables|Default|GetBuildingMesh)))
  (bind _returnvalue_2 (DynamicMesh|Reset _returnvalue))
  (Utilities|Array|Clear (Variables|Default|GetTempFootprint))
  (for _array_element (Utilities|String|ParseIntoArray (Variables|Default|Getfootprint) ";")
    (Utilities|Array|Add (Variables|Default|GetTempFootprint) (Math|Vector2D|MakeVector2D (* (Math|Conversions|ToFloat(Integer) (Utilities|Array|Get(acopy) (Utilities|String|ParseIntoArray _array_element " ") 1)) -1.0) (* (Math|Conversions|ToFloat(Integer) (Utilities|Array|Get(acopy) (Utilities|String|ParseIntoArray _array_element " "))) -1.0))))
  (if (>= (Utilities|Array|Length _tempfootprint) 3)
    (Class|GeometryScriptLibraryMeshPrimitiveFunctions|AppendSimpleExtrudePolygon :TargetMesh _returnvalue_2 :Transform (Math|Transform|MakeTransform "0, 0, 0") :PolygonVertices _tempfootprint :Height (Variables|Default|Getheight_cm) :HeightSteps 1)))